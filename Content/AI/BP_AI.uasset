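; BP_AI is an AI-controlled actor Blueprint that, on BeginPlay, has its AIC_Test controller run the BT_Test behavior tree.
; It then adds its GameplayTags to itself as non-replicated loose gameplay tags and starts a short delay with nothing after it.
; An unconnected branch that would remove those tags and print a confirmation never runs.
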(event EventBeginPlay
  (AI|RunBehaviorTree (.AsAIC%20Test (Utilities|Casting|CastToAIC_Test (AI|GetAIController self))) "/Game/AI/BT_Test.BT_Test")
  (Ability|GameplayEffect|AddLooseGameplayTags self (Variables|Default|GetGameplay%20Tags))
  (Utilities|FlowControl|Delay 3.0))

(fn ConstructionScript)